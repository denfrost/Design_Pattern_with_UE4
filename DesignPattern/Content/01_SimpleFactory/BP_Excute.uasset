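; BP_Excute is a demo driver for the Simple Factory pattern, exercising a monster factory when play begins.
; On BeginPlay it spawns a BP_MonsterFactory and stores the reference.
; A sequence then requests three monsters from GetMonster, each by a different enum value, and calls SayHello on each.
; The caller selects monsters only by enum, leaving their creation to the factory.
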(event `self.ReceiveBeginPlay`
  (`|ExecutionSequence`
    (:`then_0`
      (bind _returnvalue (`|SpawnActorFromClass` "/Game/01_SimpleFactory/BP_MonsterFactory.BP_MonsterFactory_C" (`KismetMathLibrary.MakeTransform` (0.0 0.0 0.0)) "Undefined" "OverrideRootScale" null null))
      (set `self.MonsterFactory` _returnvalue))
    (:`then_1`
      (bind _monster (`/Game/01_SimpleFactory/BP_MonsterFactory.GetMonster` (`self.MonsterFactory`) "NewEnumerator0"))
      (`/Game/01_SimpleFactory/BPI_Monster.Say Hello` _monster))
    (:`then_2`
      (bind _monster_2 (`/Game/01_SimpleFactory/BP_MonsterFactory.GetMonster` (`self.MonsterFactory`) "NewEnumerator1"))
      (`/Game/01_SimpleFactory/BPI_Monster.Say Hello` _monster_2))
    (:`then_3`
      (bind _monster_3 (`/Game/01_SimpleFactory/BP_MonsterFactory.GetMonster` (`self.MonsterFactory`) "NewEnumerator2"))
      (`/Game/01_SimpleFactory/BPI_Monster.Say Hello` _monster_3))))

(fn `UserConstructionScript`)